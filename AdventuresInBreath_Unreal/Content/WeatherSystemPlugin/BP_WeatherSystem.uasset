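; Weather system actor that follows player 0 and drives sun, fog, sky, rain and snow FX, ambient audio, and weather and tree-wind material parameter collections.
; Rain, snow and day/night weights blend sunny, snowy and rainy presets through three-way lerps, reapplied every Tick and on construction.
; Optional dynamic mode picks weighted random states and fades to them by timeline.
; Optional automatic wetness and frost trail the precipitation at separate gain/loss rates.
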(event EventTick
  (params (DeltaSeconds :type Float%20%28single-precision%29))
  (Utilities|FlowControl|Sequence
    (:then_0
      ;[1 1 1] Update Frost and Wetness automatically
      (if (Variables|WeatherSystem|Dynamics|GetUseAutomaticWetAndFrost)
        (Variables|WeatherSystem|State|SetWetWeight (+ (* (Math|Float|SelectFloat (Variables|WeatherSystem|Dynamics|GetWetGainRate) (Variables|WeatherSystem|Dynamics|GetWetLossRate) (< (- (Variables|WeatherSystem|State|GetRainingWeight) (Variables|WeatherSystem|State|GetWetWeight)) 0.0)) DeltaSeconds (- (Variables|WeatherSystem|State|GetRainingWeight) (Variables|WeatherSystem|State|GetWetWeight))) (Variables|WeatherSystem|State|GetWetWeight)))
        (Variables|WeatherSystem|State|SetFrostWeight (+ (* (Math|Float|SelectFloat (Variables|WeatherSystem|Dynamics|GetFrostGainRate) (Variables|WeatherSystem|Dynamics|GetFrostLossRate) (< (- (Variables|WeatherSystem|State|GetSnowingWeight) (Variables|WeatherSystem|State|GetFrostWeight)) 0.0)) DeltaSeconds (- (Variables|WeatherSystem|State|GetSnowingWeight) (Variables|WeatherSystem|State|GetFrostWeight))) (Variables|WeatherSystem|State|GetFrostWeight)))))
    (:then_1
      (if (Variables|WeatherSystem|Dynamics|GetUse%20Dynamic%20Changing%20Weather)
        (bind _output_get (Variables|Default|Setm_weatherCounter (- (Variables|Default|Getm_weatherCounter) DeltaSeconds)))
        (if (<= _output_get 0.0)
          (Variables|Default|Setm_previousSnow (Variables|WeatherSystem|State|GetSnowingWeight))
          (Variables|Default|Setm_previousRain (Variables|WeatherSystem|State|GetRainingWeight))
          (bind (_raining _snowing _duration _transition) (CallFunction|GetRandomWeatherState))
          (Variables|Default|Setm_weatherCounter _duration)
          (Components|Timeline|SetPlayRate (Variables|Default|GetTransitionWeightTimeline) (/ 2e+01 _transition))
          (bind _weight (Timeline|TransitionWeightTimeline PlayFromStart)
            (:Update
              (Variables|WeatherSystem|State|SetRainingWeight (Math|Float|Lerp (Variables|Default|Getm_previousRain) _raining _weight))
              (Variables|WeatherSystem|State|SetSnowingWeight (Math|Float|Lerp (Variables|Default|Getm_previousSnow) _snowing _weight)))))
        (else
          (Variables|Default|Setm_weatherCounter -1.0))))
    (:then_2
      (CallFunction|UpdateSounds)
      (CallFunction|UpdateWeatherSystem))
    (:then_3
      (Transformation|SetWorldLocation (Variables|Default|GetDefaultSceneRoot) (Transformation|GetActorLocation (Game|Player|GetPlayerPawn 0)) false false))))

(event EventBeginPlay
  (Variables|/Engine/EngineSky/BP_Sky_Sphere.BP_Sky_Sphere_C|SetDirectional%20light%20actor (Variables|Default|GetSky%20Sphere) 0)
  (if (Variables|WeatherSystem|Dynamics|GetUse%20Dynamic%20Changing%20Weather)
    (bind (_raining _snowing _duration) (CallFunction|GetRandomWeatherState))
    (bind _output_get (Variables|WeatherSystem|State|SetRainingWeight _raining))
    (Variables|WeatherSystem|State|SetWetWeight _output_get)
    (bind _output_get_2 (Variables|WeatherSystem|State|SetSnowingWeight _snowing))
    (Variables|WeatherSystem|State|SetFrostWeight _output_get_2)))

(fn ConstructionScript
  (if (Variables|WeatherSystem|Dynamics|GetUseAutomaticWetAndFrost)
    (Variables|WeatherSystem|State|SetFrostWeight (Variables|WeatherSystem|State|GetSnowingWeight))
    (Variables|WeatherSystem|State|SetWetWeight (Variables|WeatherSystem|State|GetRainingWeight)))
  (if (Variables|WeatherSystem|Dynamics|GetUse%20Dynamic%20Changing%20Weather)
    (Variables|WeatherSystem|Dynamics|SetUseAutomaticWetAndFrost true))
  (CallFunction|UpdateWeatherSystem))

(fn ThreeWayLerp
  (params (A :type Float%20%28double-precision%29) (B :type Float%20%28double-precision%29) (C :type Float%20%28double-precision%29) (B%20Weight :type Float%20%28double-precision%29) (C%20Weight :type Float%20%28double-precision%29))
  (return (Math|Float|Lerp (Math|Float|Lerp B C (Math|Float|SafeDivide C%20Weight (+ B%20Weight C%20Weight))) A (* (- 1.0 B%20Weight) (- 1.0 C%20Weight)))))

(fn ThreeWayColorLerp
  (params (A :type Linear%20Color%20Structure) (B :type Linear%20Color%20Structure) (C :type Linear%20Color%20Structure) (B%20Weight :type Float%20%28double-precision%29) (C%20Weight :type Float%20%28double-precision%29))
  (return (Math|Color|Lerp(LinearColor) (Math|Color|Lerp(LinearColor) B C (Math|Float|SafeDivide C%20Weight (+ B%20Weight C%20Weight))) A (* (- 1.0 B%20Weight) (- 1.0 C%20Weight)))))

(fn InverseWindowLerp
  (params (A :type Vector%202D%20Structure) (B :type Vector%202D%20Structure) (t :type Float%20%28double-precision%29))
  (bind _returnvalue (- t (.x B)))
  (bind _returnvalue_2 (- (.y B) (.x B)))
  (bind _returnvalue_3 (Math|Float|SafeDivide _returnvalue _returnvalue_2))
  (bind _returnvalue_4 (Math|Float|Clamp(Float) _returnvalue_3))
  (return (Math|Float|SelectFloat (Math|Float|Clamp(Float) (Math|Float|SafeDivide (- t (.x A)) (- (.y A) (.x A)))) (- 1.0 _returnvalue_4) (== _returnvalue_4 0.0))))

(fn ExponentialInterpolate
  (params (A :type Float%20%28double-precision%29) (B :type Float%20%28double-precision%29) (Alpha :type Float%20%28double-precision%29) (Exponent :type Float%20%28double-precision%29))
  (return (Math|Float|Lerp A B (Math|Float|Power Alpha Exponent))))

(fn GetDayWeight
  (return (CallFunction|InverseWindowLerp "(X=0.150000,Y=0.300000)" "(X=0.700000,Y=0.850000)" (Variables|WeatherSystem|State|GetNightDayWeight))))

(fn SkewUpWeight
  (params (Skewer :type Float%20%28double-precision%29) (Base :type Float%20%28double-precision%29) (Weight :type Float%20%28double-precision%29))
  (return (+ (* (Math|Float|Max(Float) (- Skewer Base) 0.0) Weight) Base)))

(fn UpdateDirectionalLight
  ;[1 1 1] Set Sun direction
  (Transformation|SetActorRelativeRotation (Variables|Default|GetDirectional%20Light) (Math|Rotator|MakeRotator 1.8e+02 (* (+ (Variables|WeatherSystem|State|GetNightDayWeight) 0.25) 3.6e+02) 1.8e+02))
  ;[1 1 1] Set Temperature
  (Class|LightComponent|SetTemperature (Variables|/Script/Engine.Light|GetLightComponent (Variables|Default|GetDirectional%20Light)) (Math|Float|Lerp (Variables|DayNightLighting|GetNightSunTemperature) (Variables|DayNightLighting|GetDaySunTemperature) (* (CallFunction|GetDayWeight) (- 1.0 (Variables|WeatherSystem|State|GetSnowingWeight)) (- 1.0 (Variables|WeatherSystem|State|GetRainingWeight)))))
  ;[1 1 1] Set Sun Intensity
  (Rendering|Components|Light|SetIntensity (Variables|/Script/Engine.Light|GetLightComponent (Variables|Default|GetDirectional%20Light)) (CallFunction|ThreeWayLerp (Variables|WeatherSystem|Sunny|GetSunnySunIntensity) (Variables|WeatherSystem|Snow|GetSnowSunIntensity) (Variables|WeatherSystem|Rain|GetRainSunIntensity) (Math|Float|Power (Variables|WeatherSystem|State|GetSnowingWeight) 0.3) (Math|Float|Power (Variables|WeatherSystem|State|GetRainingWeight) 0.3)))
  (Default|UpdateSunDirection (Variables|Default|GetSky%20Sphere)))

(fn UpdateFog
  (bind _frostweight (Variables|WeatherSystem|State|GetFrostWeight))
  (bind _rainingweight (Variables|WeatherSystem|State|GetRainingWeight))
  (bind _wetweight (Variables|WeatherSystem|State|GetWetWeight))
  (bind _snowingweight (Variables|WeatherSystem|State|GetSnowingWeight))
  (bind _returnvalue (CallFunction|SkewUpWeight _frostweight _snowingweight 0.3))
  (bind _returnvalue_2 (CallFunction|SkewUpWeight _wetweight _rainingweight 0.3))
  ;[1 1 1] Set Fog Density
  (Class|ExponentialHeightFogComponent|SetFogDensity (Variables|Default|GetExponentialHeightFog) (CallFunction|ThreeWayLerp (Variables|WeatherSystem|Sunny|GetSunnyFogDensity) (Variables|WeatherSystem|Snow|GetSnowFogDensity) (Variables|WeatherSystem|Rain|GetRainFogDensity) _returnvalue _returnvalue_2))
  ;[1 1 1] Set Heigh Falloff
  (Class|ExponentialHeightFogComponent|SetFogHeightFalloff (Variables|Default|GetExponentialHeightFog) (CallFunction|ThreeWayLerp (Variables|WeatherSystem|Sunny|GetSunnyFogFalloff) (Variables|WeatherSystem|Snow|GetSnowFogFalloff) (Variables|WeatherSystem|Rain|GetRainFogFalloff) _returnvalue _returnvalue_2)))

(fn UpdateFXSystems
  ;[1 1 1] Snow Flakes
  (Effects|Components|ParticleSystem|SetFloatParameter (Variables|Default|GetSnow%20FX) "SnowNumber" (Math|Float|Lerp 0.0 (Variables|WeatherSystem|Snow|GetMaxSnowParticles_Flakes) (Math|Float|Power (Variables|WeatherSystem|State|GetSnowingWeight) 1.5)))
  ;[1 1 1] Rain Droplets (no collision splash)
  (Effects|Components|ParticleSystem|SetFloatParameter (Variables|Default|GetRain%20FX) "SpawnRate" (Math|Float|Lerp 0.0 (Variables|WeatherSystem|Rain|GetMaxRainParticles_Droplets) (Variables|WeatherSystem|State|GetRainingWeight)))
  ;[1 1 1] Rain Splash Drops (collision splash)
  (Effects|Components|ParticleSystem|SetFloatParameter (Variables|Default|GetRain%20FX) "SpawnRate_02" (Math|Float|Lerp 0.0 (Variables|WeatherSystem|Rain|GetMaxRainParticles_SplashDrops) (Variables|WeatherSystem|State|GetRainingWeight)))
  ;[1 1 1] Fog Gusts
  (Effects|Components|ParticleSystem|SetFloatParameter (Variables|Default|GetRain%20FX) "SpawnRate_Fog" (CallFunction|ThreeWayLerp 0.0 (Variables|WeatherSystem|Snow|GetMaxSnowParticles_Fog) (Variables|WeatherSystem|Rain|GetMaxRainParticles_Fog) (Math|Float|Power (Variables|WeatherSystem|State|GetSnowingWeight) 3.0) (Math|Float|Power (Variables|WeatherSystem|State|GetRainingWeight) 3.0))))

(fn UpateWindMPC
  ;[1 1 1] Set Wind Intensity
  (Rendering|Material|SetScalarParameterValue "/Game/WeatherSystemPlugin/MPC/MPC_Tree_Wind.MPC_Tree_Wind" "WindRoll_Intensity" (* (CallFunction|ThreeWayLerp (Variables|WeatherSystem|Sunny|GetSunnyWindIntensity) (Variables|WeatherSystem|Snow|GetSnowWindIntensity) (Variables|WeatherSystem|Rain|GetRainWindIntensity) (Variables|WeatherSystem|State|GetSnowingWeight) (Variables|WeatherSystem|State|GetRainingWeight)) (Variables|WeatherSystem|State|GetWindIntensityWeight)) :!class /Script/Engine.KismetMaterialLibrary)
  ;[1 1 1] Set Wind Intensity
  (Rendering|Material|SetScalarParameterValue "/Game/WeatherSystemPlugin/MPC/MPC_Tree_Wind.MPC_Tree_Wind" "Wind_Weight" (* (CallFunction|ThreeWayLerp (Variables|WeatherSystem|Sunny|GetSunnyWindWeight) (Variables|WeatherSystem|Snow|GetSnowWindWeight) (Variables|WeatherSystem|Rain|GetRainWindWeight) (Variables|WeatherSystem|State|GetSnowingWeight) (Variables|WeatherSystem|State|GetRainingWeight)) (Variables|WeatherSystem|State|GetWindWeigthWeight)) :!class /Script/Engine.KismetMaterialLibrary)
  ;[1 1 1] Set Wind Intensity
  (Rendering|Material|SetScalarParameterValue "/Game/WeatherSystemPlugin/MPC/MPC_Tree_Wind.MPC_Tree_Wind" "Wind_Speed" (* (CallFunction|ThreeWayLerp (Variables|WeatherSystem|Sunny|GetSunnyWindSpeed) (Variables|WeatherSystem|Snow|GetSnowWindSpeed) (Variables|WeatherSystem|Rain|GetRainWindSpeed) (Variables|WeatherSystem|State|GetSnowingWeight) (Variables|WeatherSystem|State|GetRainingWeight)) (Variables|WeatherSystem|State|GetWindSpeedWeight)) :!class /Script/Engine.KismetMaterialLibrary))

(fn UpdateWeatherMPC
  (bind _returnvalue (CallFunction|GetDayWeight))
  (bind _snowingweight (Variables|WeatherSystem|State|GetSnowingWeight))
  (bind _rainingweight (Variables|WeatherSystem|State|GetRainingWeight))
  (bind _returnvalue_2 (- 1.0 _returnvalue))
  (bind _returnvalue_3 (- 1.0 _snowingweight))
  (bind _returnvalue_4 (- 1.0 _rainingweight))
  (bind _returnvalue_5 (* _returnvalue_2 _returnvalue_3 _returnvalue_4))
  ;[1 1 1] Set SnowBlendBias
  (Rendering|Material|SetScalarParameterValue "/Game/WeatherSystemPlugin/MPC/MPC_Weather.MPC_Weather" "SnowBlendBias" (CallFunction|ExponentialInterpolate 0.0 (Variables|WeatherSystem|Snow|GetMaxMaterialSnowBlendBias) (* (Variables|WeatherSystem|State|GetSnowingWeight) (Math|Float|Sqrt (Variables|WeatherSystem|State|GetFrostWeight))) 0.4) :!class /Script/Engine.KismetMaterialLibrary)
  ;[1 1 1] Set SnowBlend
  (Rendering|Material|SetScalarParameterValue "/Game/WeatherSystemPlugin/MPC/MPC_Weather.MPC_Weather" "SnowBlend" (Math|Float|Lerp 0.0 (Variables|WeatherSystem|Snow|GetMaxMaterialSnowBlend) (CallFunction|SkewUpWeight (Variables|WeatherSystem|State|GetSnowingWeight) (Variables|WeatherSystem|State|GetFrostWeight) 0.4)) :!class /Script/Engine.KismetMaterialLibrary)
  ;[1 1 1] Set WaterFrozen
  (Rendering|Material|SetScalarParameterValue "/Game/WeatherSystemPlugin/MPC/MPC_Weather.MPC_Weather" "WaterFrozen" (Math|Float|Lerp 0.0 1e+03 (Variables|WeatherSystem|State|GetFrostWeight)) :!class /Script/Engine.KismetMaterialLibrary)
  ;[1 1 1] Set Ripples
  (Rendering|Material|SetScalarParameterValue "/Game/WeatherSystemPlugin/MPC/MPC_Weather.MPC_Weather" "RainDropsBlend" (Math|Float|Lerp 0.0 (Variables|WeatherSystem|Rain|GetMaxMatieralRainRipples) (Variables|WeatherSystem|State|GetRainingWeight)) :!class /Script/Engine.KismetMaterialLibrary)
  ;[1 1 1] Set Roughness
  (Rendering|Material|SetScalarParameterValue "/Game/WeatherSystemPlugin/MPC/MPC_Weather.MPC_Weather" "Roughness" (Math|Float|Lerp 1.0 (Variables|WeatherSystem|Rain|GetMaxMatieralRainRoughness) (Variables|WeatherSystem|State|GetWetWeight)) :!class /Script/Engine.KismetMaterialLibrary)
  ;[1 1 1] Set Specular
  (Rendering|Material|SetScalarParameterValue "/Game/WeatherSystemPlugin/MPC/MPC_Weather.MPC_Weather" "Specular" (Math|Float|Lerp 1.0 (Variables|WeatherSystem|Rain|GetMaxMatieralRainSpecular) (Variables|WeatherSystem|State|GetWetWeight)) :!class /Script/Engine.KismetMaterialLibrary)
  ;[1 1 1] Set StarsMask
  (Rendering|Material|SetScalarParameterValue "/Game/WeatherSystemPlugin/MPC/MPC_Weather.MPC_Weather" "StarsMask" (Math|Float|Lerp 0.0 3.0 _returnvalue_5) :!class /Script/Engine.KismetMaterialLibrary)
  ;[1 1 1] Set CloudDisapear
  (Rendering|Material|SetScalarParameterValue "/Game/WeatherSystemPlugin/MPC/MPC_Weather.MPC_Weather" "CloudDisappear" (Math|Float|Lerp 0.0 1.0 _returnvalue_5) :!class /Script/Engine.KismetMaterialLibrary)
  ;[1 1 1] Set CloudColor
  (Rendering|Material|SetVectorParameterValue "/Game/WeatherSystemPlugin/MPC/MPC_Weather.MPC_Weather" "CloudColor" (CallFunction|ThreeWayColorLerp (Variables|WeatherSystem|Sunny|GetSunnyCloudColor) (Variables|WeatherSystem|Snow|GetSnowCloudColor) (Variables|WeatherSystem|Rain|GetRainCloudColor) (Math|Float|Sqrt (Variables|WeatherSystem|State|GetSnowingWeight)) (Math|Float|Sqrt (Variables|WeatherSystem|State|GetRainingWeight))) :!class /Script/Engine.KismetMaterialLibrary)
  ;[1 1 1] Set CloudColor
  (Rendering|Material|SetVectorParameterValue "/Game/WeatherSystemPlugin/MPC/MPC_Weather.MPC_Weather" "RainColor" (Math|Color|Lerp(LinearColor) (Variables|WeatherSystem|Rain|GetRainColorNight) (Variables|WeatherSystem|Rain|GetRainColorDay) (CallFunction|GetDayWeight)) :!class /Script/Engine.KismetMaterialLibrary)
  ;[1 1 1] Set CloudColor
  (Rendering|Material|SetVectorParameterValue "/Game/WeatherSystemPlugin/MPC/MPC_Weather.MPC_Weather" "SnowColor" (Math|Color|Lerp(LinearColor) (Variables|WeatherSystem|Snow|GetSnowColorNight) (Variables|WeatherSystem|Snow|GetSnowColorDay) (CallFunction|GetDayWeight)) :!class /Script/Engine.KismetMaterialLibrary))

(fn UpdateSkyLightandAtmosphere
  (bind _sunnycloudcolor (Variables|WeatherSystem|Sunny|GetSunnyCloudColor))
  (bind _snowingweight (Variables|WeatherSystem|State|GetSnowingWeight))
  (bind _snowcloudcolor (Variables|WeatherSystem|Snow|GetSnowCloudColor))
  (bind _raincloudcolor (Variables|WeatherSystem|Rain|GetRainCloudColor))
  (bind _rainingweight (Variables|WeatherSystem|State|GetRainingWeight))
  (bind _returnvalue (CallFunction|ThreeWayColorLerp _sunnycloudcolor _snowcloudcolor _raincloudcolor _snowingweight _rainingweight))
  (Class|ExponentialHeightFogComponent|SetFogInscatteringColor (Variables|Default|GetExponentialHeightFog) _returnvalue)
  (Class|SkyAtmosphereComponent|SetSkyLuminanceFactor (Variables|Default|GetSkyAtmosphere) _returnvalue)
  ;[1 1 1] Set Sky Intensity
  (Rendering|Components|Light|SetIntensity (Variables|Default|GetSkyLight) (CallFunction|ThreeWayLerp (Math|Float|Lerp (Variables|DayNightLighting|GetNightSkyLightIntensity) (Variables|DayNightLighting|GetDaySkyLightIntensity) (CallFunction|GetDayWeight)) (Variables|WeatherSystem|Snow|GetSnowSkyIntensity) (Variables|WeatherSystem|Rain|GetRainSkyIntensity) (Math|Float|Power (Variables|WeatherSystem|State|GetSnowingWeight) 0.5) (Math|Float|Power (Variables|WeatherSystem|State|GetRainingWeight) 0.5))))

(fn GetRandomWeatherState
  (bind _returnvalue (Math|Random|RandomFloat))
  (bind _weather_switch_random (Variables|WeatherSystem|Dynamics|GetWeather%20Switch%20Random))
  (bind _cansunny (Variables|WeatherSystem|Dynamics|GetCanSunny))
  (bind _canrain (Variables|WeatherSystem|Dynamics|GetCanRain))
  (bind _cansnow (Variables|WeatherSystem|Dynamics|GetCanSnow))
  (bind _canrainsnow (Variables|WeatherSystem|Dynamics|GetCanRainSnow))
  (bind _returnvalue_2 (+ _cansunny _canrain _cansnow _canrainsnow))
  (bind _returnvalue_3 (+ _cansunny _canrain))
  (bind _returnvalue_4 (/ _cansunny _returnvalue_2))
  (bind _returnvalue_5 (/ _returnvalue_3 _returnvalue_2))
  (bind _returnvalue_6 (< _returnvalue _returnvalue_4))
  (bind _returnvalue_7 (< _returnvalue _returnvalue_5))
  (bind _returnvalue_8 (not _returnvalue_6))
  (return (Math|Float|SelectFloat (Math|Random|RandomFloatinRange 0.3 1.0) 0.0 (and _returnvalue_8 (or _returnvalue_7 (not (< _returnvalue (/ (+ _returnvalue_3 _cansnow) _returnvalue_2)))))) (Math|Float|SelectFloat (Math|Random|RandomFloatinRange 0.3 1.0) 0.0 (and _returnvalue_8 (not _returnvalue_7))) (Math|Random|RandomFloatinRange (.x _weather_switch_random) (.y _weather_switch_random)) (/ (Math|Random|RandomFloatinRange 0.0 (.x (Variables|WeatherSystem|Dynamics|GetWeather%20Switch%20Random))) 2.5)))

(fn UpdateWeatherSystem
  (CallFunction|UpdateDirectionalLight)
  (CallFunction|UpdateFog)
  (CallFunction|UpdateFXSystems)
  (CallFunction|UpateWindMPC)
  (CallFunction|UpdateWeatherMPC)
  (CallFunction|UpdateSkyLightandAtmosphere))

(fn UpdateSounds
  (bind _returnvalue (CallFunction|GetDayWeight))
  (bind _rainingweight (Variables|WeatherSystem|State|GetRainingWeight))
  (bind _snowingweight (Variables|WeatherSystem|State|GetSnowingWeight))
  (bind _returnvalue_2 (- 1.0 _rainingweight))
  (bind _returnvalue_3 (- 1.0 _snowingweight))
  (bind _returnvalue_4 (* _returnvalue_3 _returnvalue_2))
  (bind _returnvalue_5 (* _returnvalue _returnvalue_4))
  (if (Variables|Default|GetUseSound)
    (Audio|Components|Audio|SetVolumeMultiplier (Variables|Default|GetRain%20Audio) (Variables|WeatherSystem|State|GetRainingWeight) :!class /Script/Engine.AudioComponent)
    (Audio|Components|Audio|SetVolumeMultiplier (Variables|Default|GetSnow%20Audio) (Variables|WeatherSystem|State|GetSnowingWeight) :!class /Script/Engine.AudioComponent)
    (Audio|Components|Audio|SetVolumeMultiplier (Variables|Default|GetBirds%20Audio) _returnvalue_5 :!class /Script/Engine.AudioComponent)
    (Audio|Components|Audio|SetVolumeMultiplier (Variables|Default|GetCicada%20Audio) _returnvalue_5 :!class /Script/Engine.AudioComponent)
    (Audio|Components|Audio|SetVolumeMultiplier (Variables|Default|GetWind%20Audio) (Math|Float|Lerp 0.25 1.0 (- 1.0 _returnvalue_4)) :!class /Script/Engine.AudioComponent)))

(fn ThreeWayExpoLerp
  (params (A :type Float%20%28double-precision%29) (B :type Float%20%28double-precision%29) (C :type Float%20%28double-precision%29) (B%20Weight :type Float%20%28double-precision%29) (B%20Pow :type Float%20%28double-precision%29) (C%20Weight :type Float%20%28double-precision%29) (C%20Pow :type Float%20%28double-precision%29))
  (return (Math|Float|Lerp (Math|Float|Lerp B C (Math|Float|SafeDivide C%20Weight (+ B%20Weight C%20Weight))) A (* (- 1.0 B%20Weight) (- 1.0 C%20Weight)))))